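; BP_Character is a character Blueprint that moves on input and fires projectiles on a left mouse click.
; The MoveForward and MoveRight axis events feed movement input along the capsule component's forward and right vectors.
; Each click spawns a BP_Projectile at SpawnDistance ahead of the actor along the capsule's forward vector.
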(event `Key|LeftMouseButton`
  (params (Key :type "Key Structure"))
  (:`Pressed`
    (`|SpawnActorFromClass` "/Game/Blueprints/BP_Projectile.BP_Projectile_C" (`KismetMathLibrary.MakeTransform` (+ (`self.K2_GetActorLocation`) (* (`SceneComponent.GetForwardVector` (`self.CapsuleComponent`)) (`self.SpawnDistance`)))) "Undefined" "OverrideRootScale" null null)))

(event `InputAxis|MoveForward`
  (params (AxisValue :type "Float (single-precision)"))
  (`self.AddMovementInput` (* AxisValue (`SceneComponent.GetForwardVector` (`self.CapsuleComponent`)))))

(event `InputAxis|MoveRight`
  (params (AxisValue :type "Float (single-precision)"))
  (`self.AddMovementInput` (* AxisValue (`SceneComponent.GetRightVector` (`self.CapsuleComponent`)))))

(fn `UserConstructionScript`)