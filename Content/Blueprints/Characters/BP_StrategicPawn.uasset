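; BP_StrategicPawn is an RTS-style player pawn with free camera movement, mouse selection and army commands.
; On BeginPlay it spawns a BP_Army and caches BP_HUD, which shows the left-drag box while camera rotation pauses.
; Releasing deprojects the corners to query MESubsystem for SelectedEntities.
; Right-click sets the army center and spawns a SteeringEntity there; Space calls ShouldMoveToLocation(true), with a Ctrl-held gate adding a false call.
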(event `self.ReceiveBeginPlay`
  (bind _returnvalue (`self.GetTransform`))
  (set `PlayerController.bShowMouseCursor` true (`GameplayStatics.GetPlayerController` 0))
  (bind _returnvalue_2 (`|SpawnActorFromClass` "/Game/Blueprints/Actors/BP_Army.BP_Army_C" (`KismetMathLibrary.MakeTransform` (`KismetMathLibrary.MakeVector` (.x (.location _returnvalue)) (.y (.location _returnvalue)))) "AlwaysSpawn" "OverrideRootScale" self null))
  (set `self.Army` _returnvalue_2)
  (bind _asbp_hud (cast `/Game/Blueprints/UI/BP_HUD` (`PlayerController.GetHUD` (`GameplayStatics.GetPlayerController` 0)))
    (:`then`
      (set `self.HUD` _asbp_hud))
    (:`CastFailed`
      (`KismetSystemLibrary.PrintString` "Failed to set HUD" true true (struct :`R` 1.0 :`G` 0.030793 :`A` 1.0) 10.0))))

(event `InputAxis|MoveForward`
  (params (AxisValue :type "Float (single-precision)"))
  (`self.K2_AddActorWorldTransform` (`KismetMathLibrary.MakeTransform` (* (* AxisValue (`KismetMathLibrary.GetForwardVector` (`self.GetControlRotation`))) (`self.MoveSpeed`))) true))

(event `InputAxis|MoveRight`
  (params (AxisValue :type "Float (single-precision)"))
  (`self.K2_AddActorWorldTransform` (`KismetMathLibrary.MakeTransform` (* (* AxisValue (`KismetMathLibrary.GetRightVector` (`self.GetControlRotation`))) (`self.MoveSpeed`))) true))

(event `InputAxis|LookUp`
  (params (AxisValue :type "Float (single-precision)"))
  (if (`self.bShouldControllerRotate`)
    (`self.AddControllerPitchInput` AxisValue)))

(event `InputAxis|LookRight`
  (params (AxisValue :type "Float (single-precision)"))
  (if (`self.bShouldControllerRotate`)
    (`self.AddControllerYawInput` AxisValue)))

(event `Key|LeftMouseButton`
  (params (Key :type "Key Structure"))
  (bind _returnvalue (`GameplayStatics.GetPlayerController` 0))
  (bind _hud (`self.HUD`))
  (bind (_locationx _locationy) (`PlayerController.GetMousePosition` (`GameplayStatics.GetPlayerController` 0)))
  (bind (_locationx_2 _locationy_2) (`PlayerController.GetMousePosition` _returnvalue))
  (bind (_mousestartposition_x _mousestartposition_y) (`KismetMathLibrary.BreakVector2D` (`/Game/Blueprints/UI/BP_HUD.MouseStartPosition` _hud)))
  (bind (_worldposition _worlddirection) (`GameplayStatics.DeprojectScreenToWorld` _returnvalue (`KismetMathLibrary.MakeVector2D` _locationx_2 _locationy_2)))
  (:`Pressed`
    (set `self.bShouldControllerRotate` false)
    (set `/Game/Blueprints/UI/BP_HUD.bShouldDraw` true _hud)
    (`/Game/Blueprints/UI/BP_HUD.Draw Rect` _hud _locationx _locationy)
    (set `self.Point1` (`GameplayStatics.DeprojectScreenToWorld` (`GameplayStatics.GetPlayerController` 0) (`KismetMathLibrary.MakeVector2D` _mousestartposition_x _mousestartposition_y))))
  (:`Released`
    (set `self.bShouldControllerRotate` true)
    (set `/Game/Blueprints/UI/BP_HUD.bShouldDraw` false (`self.HUD`))
    (bind _outentities (`MESubsystem.GetEntitiesInsideRect` (subsystem `MESubsystem`) (`self.Point1`) (+ _worldposition (* _worlddirection (`self.Distance`)))))
    (set `self.SelectedEntities` _outentities)))

(event `Key|RightMouseButton`
  (params (Key :type "Key Structure"))
  (bind _hitresult (`PlayerController.GetHitResultUnderCursorByChannel` (`GameplayStatics.GetPlayerController` 0) "TraceTypeQuery1" true))
  (:`Pressed`
    (`KismetSystemLibrary.DrawDebugSphere` (`.ImpactPoint` (`GameplayStatics.BreakHitResult` _hitresult)) 300.0 12 (struct :`R` 0.317237 :`G` 0.169797 :`B` 1.0 :`A` 1.0) 2.0 10.0)
    (`MEArmy.SetArmyCenter` (`self.Army`) (`.ImpactPoint` (`GameplayStatics.BreakHitResult` _hitresult)))
    (`MESubsystem.SpawnEntity` (subsystem `MESubsystem`) "SteeringEntity" self (`.ImpactPoint` (`GameplayStatics.BreakHitResult` _hitresult)))))

(event `Key|SpaceBar`
  (params (Key :type "Key Structure"))
  (:`Pressed`
    (`MEArmy.ShouldMoveToLocation` (`self.Army`) true)))

(event `Key|SpaceBar`
  (params (Key :type "Key Structure"))
  (:`Pressed`
    (`/Engine/EditorBlueprintResources/StandardMacros.Gate` true :!label _label
      (:`Exit`
        (`MEArmy.ShouldMoveToLocation` (`self.Army`) false)))))

(event `Key|LeftControl`
  (params (Key :type "Key Structure"))
  (:`Pressed`
    (goto _label :!via `Open`))
  (:`Released`
    (goto _label :!via `Close`)))

(fn `UserConstructionScript`)