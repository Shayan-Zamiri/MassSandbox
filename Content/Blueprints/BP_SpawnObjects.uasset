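; BP_SpawnObjects fills a square grid with mesh instances when play begins.
; Nested loops add instances to a single InstancedStaticMesh component, spacing them along X and Y by the Size variable.
; An unconnected duplicate of the loops would spawn a separate BP_SMActor at each grid point instead, but it never runs.
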(event `self.ReceiveBeginPlay`
  (bind _size (`self.Size`))
  (for _index (range 101)
    (for _index_2 (range 101)
      (`InstancedStaticMeshComponent.AddInstance` (`self.InstancedStaticMesh`) (`KismetMathLibrary.MakeTransform` (`KismetMathLibrary.MakeVector` (* (`KismetMathLibrary.Conv_IntToDouble` _index) _size) (* (`KismetMathLibrary.Conv_IntToDouble` _index_2) _size))) false))))

(fn `UserConstructionScript`)